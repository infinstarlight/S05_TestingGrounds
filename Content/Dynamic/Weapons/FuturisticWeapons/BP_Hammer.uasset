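; BP_Hammer is a hammer weapon pickup with a rotating movement component.
; On overlap with its pickup collision, it looks up its named row in the weapon data table, adds it to MyWeapons and stops the movement.
; If the overlapping actor is BP_Character, it calls FindFirstFreeSlot on it without using a result, prints a debug string and destroys itself.
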(event OnComponentBeginOverlap(PickupCollision)
  (params (OverlappedComponent :type Primitive%20Component%20Object%20Reference) (OtherActor :type Actor%20Object%20Reference) (OtherComp :type Primitive%20Component%20Object%20Reference) (OtherBodyIndex :type Integer) (bFromSweep :type Boolean) (SweepResult :type Hit%20Result%20Structure%20%28by%20ref%29))
  (CallFunction|OnPickup (Variables|Default|GetName))
  (Components|Movement|StopMovementImmediately (Variables|Default|GetRotatingMovement))
  (bind _asbp_character (Utilities|Casting|CastToBP_Character OtherActor))
  (Default|FindFirstFreeSlot _asbp_character)
  (Development|PrintString "Hello")
  (Actor|DestroyActor))

(event Custom|OnPickup
  (params (Name :type Name))
  (bind _returnvalue (Utilities|GetDataTableRow "/Game/Dynamic/Game/Weapon_DataTable.Weapon_DataTable" Name)
    (:then
      (bind _output_get (Variables|Default|SetHammer%20Var _returnvalue))
      (Utilities|Array|AddUnique (Variables|Default|GetMy%20Weapons) _output_get))))

(event EventBeginPlay)

(event Collision|EventActorBeginOverlap
  (params (OtherActor :type Actor%20Object%20Reference)))

(event EventTick
  (params (DeltaSeconds :type Float%20%28single-precision%29)))

(fn ConstructionScript)