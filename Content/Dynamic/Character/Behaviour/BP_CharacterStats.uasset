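; BP_CharacterStats is a character behaviour Blueprint that tracks health.
; BeginPlay sets CurrentHealth to MaxHealth, and TakeDamage subtracts damage from it, clamped between zero and MaxHealth.
; GetHealth returns the current value, while IsDead is an empty stub, so nothing here reacts to health reaching zero.
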(event EventBeginPlay
  (Variables|PlayerStats|SetCurrentHealth (Variables|Default|GetMaxHealth)))

(event EventTick
  (params (DeltaSeconds :type Float%20%28single-precision%29)))

(fn TakeDamage
  (params (Damage :type Float%20%28single-precision%29))
  (Variables|PlayerStats|SetCurrentHealth (Math|Float|Clamp(Float) (- (Variables|PlayerStats|GetCurrentHealth) Damage) 0.0 (Variables|Default|GetMaxHealth))))

(fn GetHealth
  (return (Variables|PlayerStats|GetCurrentHealth)))

(fn IsDead)