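; BP_BaseWeapon is a base weapon that fires projectiles from a limited ammo count, refilled to maximum on BeginPlay or through Reload.
; Shoot spawns the configured projectile class at a supplied transform with the owning Pawn as instigator, then decrements ammo.
; An empty magazine or non-Pawn owner blocks firing and prints a message; the file itself binds no input.
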(event EventBeginPlay
  (CallFunction|Reload))

(event EventTick
  (params (DeltaSeconds :type Float%20%28single-precision%29)))

(fn Reload
  (Variables|Default|SetCurrentAmmo (Variables|Default|GetMaxAmmo)))

(fn Shoot
  (params (Transform :type Transform))
  (if (> (Variables|Default|GetCurrentAmmo) 0)
    (bind _aspawn (Utilities|Casting|CastToPawn (Components|GetOwner))
      (:then
        (Game|SpawnActorfromClass (Variables|Default|GetProjectileType) Transform "Undefined" 0 _aspawn)
        (bind _result (Math|Integer|DecrementInt (Variables|Default|GetCurrentAmmo))
          (:%20%20
            (Variables|Default|SetCurrentAmmo _result))))
      (:CastFailed
        (Development|PrintString "Unable to Shoot from non-pawn")))
    (else
      (Development|PrintString "No Ammo. Press R to Reload!"))))