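; Player controller Blueprint that forwards Fire, Reload and Jump input to the possessed BP_Character.
; Fire and Reload trigger the character's attack and reload; Jump starts and stops jumping while tracking button state in IsJumpButtonDown.
; Both jump events then check movement velocity to set JumpZVelocity, though moving and stationary branches assign the same value.
; Jump release reuses the character cast made on press.
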(event EventBeginPlay)

(event EventTick
  (params (DeltaSeconds :type Float%20%28single-precision%29)))

(event Input|ActionEvents|InputActionReload
  (params (Key :type Key%20Structure))
  (:Pressed
    (bind _asbp_character (Utilities|Casting|CastToBP_Character (Pawn|GetControlledPawn)))
    (Default|StartReload _asbp_character)))

(event Input|ActionEvents|InputActionJump
  (params (Key :type Key%20Structure))
  (:Pressed
    (bind _asbp_character (Utilities|Casting|CastToBP_Character (Pawn|GetControlledPawn)))
    (Character|Jump _asbp_character)
    (Variables|Default|SetIs%20Jump%20Button%20Down? (Character|CanJump _asbp_character))
    (bind _ascharacter_movement_component (Utilities|Casting|CastToCharacterMovementComponent (Pawn|GetMovementComponent _asbp_character) :!label _label))
    (if (> (Math|Vector|VectorLength (Variables|/Script/Engine.MovementComponent|GetVelocity _ascharacter_movement_component)) 0.0)
      (Variables|/Script/Engine.CharacterMovementComponent|SetJumpZVelocity _ascharacter_movement_component 4e+02)
      (else
        (Variables|/Script/Engine.CharacterMovementComponent|SetJumpZVelocity _ascharacter_movement_component 4e+02))))
  (:Released
    (Character|StopJumping _asbp_character)
    (Variables|Default|SetIs%20Jump%20Button%20Down? false)
    (goto _label)))

(event Input|ActionEvents|InputActionFire
  (params (Key :type Key%20Structure))
  (:Pressed
    (bind _asbp_character (Utilities|Casting|CastToBP_Character (Pawn|GetControlledPawn)))
    (Default|StartAttack _asbp_character)))

(fn ConstructionScript)